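; BP_Character is the input-handling Blueprint for a snake: it spawns a BP_SnakeHead on BeginPlay and stores it as Head.
; Four directional axis inputs move that head by local offsets, with Left/Right on Y and Forward/Backward on Z.
; Each nonzero axis event applies a fixed one-unit step without sweep, ignoring axis magnitude and frame time.
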(event `self.ReceiveBeginPlay`
  (bind _returnvalue (`|SpawnActorFromClass` "/Game/BluePrint/BP_SnakeHead.BP_SnakeHead_C" (`self.Spawn Transform`) "Undefined" "OverrideRootScale" null null))
  (set `self.Head` _returnvalue))

(event `InputAxis|Input_Left`
  (params (AxisValue :type "Float (single-precision)"))
  (if (!= AxisValue 0.0)
    (`self.K2_AddActorLocalOffset` (`self.Head`) (0.0 -1.0 0.0) false false)))

(event `InputAxis|Input_Right`
  (params (AxisValue :type "Float (single-precision)"))
  (if (!= AxisValue 0.0)
    (`self.K2_AddActorLocalOffset` (`self.Head`) (0.0 1.0 0.0) false false)))

(event `InputAxis|Input_Forward`
  (params (AxisValue :type "Float (single-precision)"))
  (if (!= AxisValue 0.0)
    (`self.K2_AddActorLocalOffset` (`self.Head`) (0.0 0.0 1.0) false false)))

(event `InputAxis|Input_Backward`
  (params (AxisValue :type "Float (single-precision)"))
  (if (!= AxisValue 0.0)
    (`self.K2_AddActorLocalOffset` (`self.Head`) (0.0 0.0 -1.0) false false)))

(fn `UserConstructionScript`)